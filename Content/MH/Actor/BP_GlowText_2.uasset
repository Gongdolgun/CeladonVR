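; BP_GlowText_2 is a text actor that shows timed Korean captions explaining the pottery wheel and celadon shaping.
; BeginPlay runs a fixed Delay chain, updating its TextRender through SetText and ending on a prompt to clear the sparkles to finish the pot's shape.
; It also finds BP_GlowText_3 with GetActorOfClass and sets matching one-word terms on it during the first two steps.
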(event EventBeginPlay
  (Utilities|FlowControl|Delay 14.0)
  (CallFunction|SetText "물레는 도자기를 만들 때 흙을 
올려서 돌려, 도자기의 모양을  
만들 수 있는 도구에요.")
  (bind _returnvalue (Actor|GetActorOfClass "/Game/MH/Actor/BP_GlowText_3.BP_GlowText_3_C"))
  (Default|SetText _returnvalue "물레")
  (Utilities|FlowControl|Delay 6.42)
  (CallFunction|SetText "성형은 청자의 모양을  
만드는 과정이에요.")
  (Default|SetText _returnvalue "성형")
  (Utilities|FlowControl|Delay 2.8)
  (CallFunction|SetText "앞에 보이는 반짝이를  
모두 없에서 도자기의  
모양을 완성해 보세요."))

(event Collision|EventActorBeginOverlap
  (params (OtherActor :type Actor%20Object%20Reference)))

(event EventTick
  (params (DeltaSeconds :type Float%20%28single-precision%29)))

(fn ConstructionScript)

(fn SetText
  (params (NewParam :type Text))
  (Rendering|Components|TextRender|SetText (Variables|Default|GetTextRender) NewParam)
  (return))